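; Spike trap obstacle that cycles up and down and stabs the first actor to overlap its death trigger.
; TrapTimeline moves SpikeWide vertically; on finishing, it pauses and reverses, with Speed scaling both play rate and pauses, and plays an attenuated strike sound on each move.
; The overlap sends StabbedMessage to that actor and sets IsDead, blocking further stabs and leaving the spikes raised once they next reach the top.
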(event OnComponentBeginOverlap(DeathTrigger)
  (params (OverlappedComponent :type Primitive%20Component%20Object%20Reference) (OtherActor :type Actor%20Object%20Reference) (OtherComp :type Primitive%20Component%20Object%20Reference) (OtherBodyIndex :type Integer) (bFromSweep :type Boolean) (SweepResult :type Hit%20Result%20Structure%20%28by%20ref%29))
  (if (not (Variables|Default|GetisDead))
    (Class|BPITrap|Stabbed(Message) OtherActor)
    (Variables|Default|SetisDead true)))

(event Custom|Rise
  (bind (_direction _spikerise) (Timeline|TrapTimeline PlayFromStart)
    (:Update
      (Transformation|SetRelativeLocation (Variables|Default|GetSpikeWide) (Math|Vector|MakeVector 0.0 0.0 (* _spikerise 2.5e+02)) false false))
    (:Finished
      (if (Utilities|Enum|Equal(Enum) _direction "Forward")
        (Utilities|FlowControl|Delay (/ 0.6 (Variables|Default|GetSpeed)))
        (if (not (Variables|Default|GetisDead))
          (CallFunction|Down)
          (CallFunction|PlayTrapSound :!label _label))
        (else
          (Utilities|FlowControl|Delay (/ 1.2 (Variables|Default|GetSpeed)))
          (CallFunction|Rise)
          (goto _label))))))

(event Custom|Down
  (bind (_direction _spikerise) (Timeline|TrapTimeline ReverseFromEnd)
    (:Update
      (Transformation|SetRelativeLocation (Variables|Default|GetSpikeWide) (Math|Vector|MakeVector 0.0 0.0 (* _spikerise 2.5e+02)) false false))
    (:Finished
      (if (Utilities|Enum|Equal(Enum) _direction "Forward")
        (Utilities|FlowControl|Delay (/ 0.6 (Variables|Default|GetSpeed)))
        (if (not (Variables|Default|GetisDead))
          (CallFunction|Down)
          (CallFunction|PlayTrapSound :!label _label))
        (else
          (Utilities|FlowControl|Delay (/ 1.2 (Variables|Default|GetSpeed)))
          (CallFunction|Rise)
          (goto _label))))))

(event EventBeginPlay
  (Variables|Default|SetWorldPosition (Transformation|GetWorldLocation (Variables|Default|GetSpikeWide)))
  (Components|Timeline|SetPlayRate (Variables|Default|GetTrapTimeline) (Variables|Default|GetSpeed))
  (CallFunction|PlayTrapSound)
  (bind (_direction _spikerise) (Timeline|TrapTimeline Play)
    (:Update
      (Transformation|SetRelativeLocation (Variables|Default|GetSpikeWide) (Math|Vector|MakeVector 0.0 0.0 (* _spikerise 2.5e+02)) false false))
    (:Finished
      (if (Utilities|Enum|Equal(Enum) _direction "Forward")
        (Utilities|FlowControl|Delay (/ 0.6 (Variables|Default|GetSpeed)))
        (if (not (Variables|Default|GetisDead))
          (CallFunction|Down)
          (CallFunction|PlayTrapSound :!label _label))
        (else
          (Utilities|FlowControl|Delay (/ 1.2 (Variables|Default|GetSpeed)))
          (CallFunction|Rise)
          (goto _label))))))

(event Collision|EventActorBeginOverlap
  (params (OtherActor :type Actor%20Object%20Reference)))

(event EventTick
  (params (DeltaSeconds :type Float%20%28single-precision%29)))

(fn ConstructionScript)

(fn PlayTrapSound
  (Audio|SpawnSoundatLocation "/Game/ObstacleGame/spike-strike-4.spike-strike-4" (Variables|Default|GetWorldPosition) "0, 0, 0" 1.0 1.0 0.0 "/Game/ObstacleGame/TrapSoundAttenuation.TrapSoundAttenuation" 0))